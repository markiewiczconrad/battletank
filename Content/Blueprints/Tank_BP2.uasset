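; Player-controllable tank Blueprint that wires its turret, barrel and track components to input for driving, aiming and firing.
; The construction script assigns part meshes and initializes TankMovement with both tracks; BeginPlay registers turret and barrel references.
; Input drives tracks directly through throttle axes or through TankMovement's move and rotate intents.
; Aim axes rotate the azimuth gimbal and spring arm, scaled by delta time, while Fire calls the firing function.
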(event `self.ReceiveBeginPlay`
  (`self.SetTurretReference` (`self.TankTurret`))
  (`self.SetBarrelReference` (`self.TankBarrel`)))

(event `InputAxis|LeftTrackThrottle`
  (params (AxisValue :type "Float (single-precision)"))
  (`TankTrack.SetThrottle` (`self.LeftTankTrack`) AxisValue))

(event `InputAxis|AimAzimuth`
  (params (AxisValue :type "Float (single-precision)"))
  (`SceneComponent.K2_AddLocalRotation` (`self.Azimuth Gimbal`) (`KismetMathLibrary.MakeRotator` 0.0 0.0 (* AxisValue (`GameplayStatics.GetWorldDeltaSeconds`) 100.0)) false false))

(event `InputAxis|RightTrackThrottle`
  (params (AxisValue :type "Float (single-precision)"))
  (`TankTrack.SetThrottle` (`self.RightTankTrack`) AxisValue))

(event `InputAxis|Move`
  (params (AxisValue :type "Float (single-precision)"))
  (`TankMovementComponent.IntendMove` (`self.TankMovement`) AxisValue))

(event `InputAxis|AimElevation`
  (params (AxisValue :type "Float (single-precision)"))
  (`SceneComponent.K2_AddLocalRotation` (`self.SpringArm`) (`KismetMathLibrary.MakeRotator` 0.0 (* AxisValue (`GameplayStatics.GetWorldDeltaSeconds`) 100.0)) false false))

(event `InputAxis|Rotate`
  (params (AxisValue :type "Float (single-precision)"))
  (`TankMovementComponent.IntendRotate` (`self.TankMovement`) AxisValue))

(event `InputAction|Fire`
  (params (Key :type "Key Structure"))
  (:`Pressed`
    (`self.Fire`)))

(fn `UserConstructionScript`
  (bind _lefttanktrack (`self.LeftTankTrack`))
  (bind _righttanktrack (`self.RightTankTrack`))
  (`StaticMeshComponent.SetStaticMesh` (`self.TankTurret`) "/Game/Models/tank_fbx_Turret.tank_fbx_Turret")
  (`StaticMeshComponent.SetStaticMesh` (`self.TankBarrel`) "/Game/Models/tank_fbx_Barrel.tank_fbx_Barrel")
  (`StaticMeshComponent.SetStaticMesh` _lefttanktrack "/Game/Models/tank_fbx_Track.tank_fbx_Track")
  (`StaticMeshComponent.SetStaticMesh` _righttanktrack "/Game/Models/tank_fbx_Track.tank_fbx_Track")
  (`TankMovementComponent.Initialize` (`self.TankMovement`) _lefttanktrack _righttanktrack))